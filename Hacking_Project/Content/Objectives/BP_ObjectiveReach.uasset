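; Interactable trigger objective that marks the end of a level as reached when the player enters it.
; On entry it shows an "END REACHED" HUD prompt, sets InteractOnce and immediately ends the interaction without any input.
; Ending the interaction fires the BPCObjectiveTarget reach-complete dispatcher, then disables the trigger and opens the hard-coded Level_2_Agathe map.
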(fn `OnInteractionEnd`
  (`parent.OnInteractionEnd`)
  (`/Game/Objectives/BPC_ObjectiveTarget.EvtDispatcher_OnReachComplete` (`self.BPC_ObjectiveTarget`))
  (if (`self.bInteractOnce`)
    (`self.EnableTrigger` false)
    (`GameplayStatics.OpenLevel` "Level_2_Agathe")))

(fn `OnInteractionStart`)

(fn `OnPlayerEnter`
  (`parent.OnPlayerEnter`)
  (`self.RefreshHUD` true)
  (`self.OnInteractionEnd`))

(fn `RefreshHUD`
  (params (bDisplay :type Boolean))
  (`parent.RefreshHUD` false)
  (`/Game/UI/WBP_PlayerHUD.DisplayInteraction` (`/Game/Player/BP_Player.HUDWidget` (`self.PlayerInTrigger`)) bDisplay (`self.bIsLocked`) "END REACHED" "")
  (set `self.bInteractOnce` true))

(fn `UserConstructionScript`
  (`parent.UserConstructionScript`))