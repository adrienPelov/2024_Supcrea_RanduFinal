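; Objective target component that marks its owning actor as complete and broadcasts a target-complete dispatcher for objectives.
; InitTarget stores the target type and binds events for Interact (the owner's BP_TriggerInteraction end) or Reach (a reach-complete dispatcher), clearing CompleteOnce.
; BeginPlay passes Collect, which has no binding case.
; OnReachComplete fires only once, while OnTargetComplete can repeat unless CompleteOnce is set; both print debug text.
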(event `self.ReceiveBeginPlay`
  (`self.InitTarget` "NewEnumerator0"))

(fn `InitTarget`
  (params (Type :type "/Game/Objectives/_Enums/EObjectiveType Enum" :default "NewEnumerator0"))
  (bind _output_get (set `self.Type` Type))
  (switch `/Game/Objectives/_Enums/EObjectiveType` _output_get
    (:`NewEnumerator1`
      (bind _asbp_trigger_interaction (cast `/Game/PlayerTriggers/BP_TriggerInteraction` (`self.GetOwner`)))
      (add `/Game/PlayerTriggers/BP_TriggerInteraction.EvtDispatcher_OnInteractionEnd` _asbp_trigger_interaction (`|CreateDelegate` :!event `OnTargetComplete`))
      (set `self.bCompleteOnce` false))
    (:`NewEnumerator2`
      (cast `/Game/PlayerTriggers/BP_TriggerInteraction` (`self.GetOwner`))
      (add `self.EvtDispatcher_OnReachComplete` (`|CreateDelegate` :!event `OnReachComplete`))
      (set `self.bCompleteOnce` false))))

(fn `OnReachComplete`
  (if (not (`self.bIsComplete`))
    (`KismetSystemLibrary.PrintString` (`KismetStringLibrary.Concat_StrStr` (`KismetSystemLibrary.GetDisplayName` (`self.GetOwner`)) " | On Target Complete"))
    (set `self.bIsComplete` true)
    (`self.EvtDispatcher_OnTargetComplete` self)))

(fn `OnTargetComplete`
  (if (`self.bCompleteOnce`)
    (if (not (`self.bIsComplete`))
      (`KismetSystemLibrary.PrintString` (`KismetStringLibrary.Concat_StrStr` (`KismetSystemLibrary.GetDisplayName` (`self.GetOwner`)) " | On Target Complete") :!label _label)
      (set `self.bIsComplete` true)
      (`self.EvtDispatcher_OnTargetComplete` self))
    (else
      (goto _label))))