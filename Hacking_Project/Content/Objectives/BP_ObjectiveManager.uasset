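; BP_ObjectiveManager runs the level's ordered list of objectives, each with a type, title, description and targets.
; At BeginPlay it registers each target's BPC_ObjectiveTarget component, then polls on Tick for the player's HUD to start the first objective.
; Target completions update the HUD count until the objective completes.
; The HUD's fade-complete event triggers the next objective or prints level complete.
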(event `self.ReceiveBeginPlay`
  (`self.InitObjectives`))

(event `self.ReceiveTick`
  (params (DeltaSeconds :type "Float (single-precision)"))
  (`self.HUDRef`
    (:`then`)
    (:`else`
      (bind _outactors (`GameplayStatics.GetAllActorsOfClass` "/Game/Player/BP_Player.BP_Player_C"))
      (bind _output (`|GetArrayItem` _outactors))
      (`/Engine/EditorBlueprintResources/StandardMacros.IsValid` _output
        (:`Is Valid`
          (bind _output_get (set `self.HUDRef` (`/Game/Player/BP_Player.HUDWidget` _output)))
          (add `/Game/UI/WBP_PlayerHUD.EvtDispatcher_ObjectiveComplete` _output_get (delegate `Evt_ObjectiveFadeComplete`))
          (`self.StartObjective` 0))))))

(event `Evt_ObjectiveFadeComplete`
  (`self.OnHUDFadeComplete`))

(fn `InitObjectives`
  (`|ExecutionSequence`
    (:`then_0`
      (set `self.CurObjectiveIndex` 0))
    (:`then_1`
      (set `self.NbTargetsComplete` 0))
    (:`then_2`
      (`KismetArrayLibrary.Array_Clear` (`self.CurTargets`)))
    (:`then_3`
      (for _array_element (`self.Objectives`)
        (bind ((`Type_7_5FB78B454A558388937C8185BD36DD93` _type) (`Targets_11_57A2790B41ECB63A723A17ABB7A00F93` _targets)) (break `/Game/Objectives/_Structs/FObjective` _array_element))
        (for _array_element_2 _targets
          (bind _returnvalue (`self.GetComponentByClass` _array_element_2 "/Game/Objectives/BPC_ObjectiveTarget.BPC_ObjectiveTarget_C"))
          (`/Engine/EditorBlueprintResources/StandardMacros.IsValid` _returnvalue
            (:`Is Valid`
              (`self.RegisterTarget` _returnvalue _type))))))))

(fn `OnHUDFadeComplete`
  (if (`self.AllObjectivesCompleted`)
    (`KismetSystemLibrary.PrintString` "Objective Manager | Level Complete!" true true (struct :`R` 1.0 :`G` 0.598144 :`A` 1.0))
    (else
      (`self.StartObjective` (`self.CurObjectiveIndex`)))))

(fn `OnObjectiveComplete`
  (`/Game/UI/WBP_PlayerHUD.CompleteObjective` (`self.HUDRef`))
  (`/Engine/EditorBlueprintResources/StandardMacros.IncrementInt` (`self.CurObjectiveIndex`)))

(fn `OnTargetComplete`
  (params (Target :type "/Game/Objectives/BPC_ObjectiveTarget Object Reference"))
  (if (`KismetArrayLibrary.Array_Contains` (`self.CurTargets`) Target)
    (`|ExecutionSequence`
      (:`then_0`
        (bind _result (`/Engine/EditorBlueprintResources/StandardMacros.IncrementInt` (`self.NbTargetsComplete`))
          (:`  `
            (`/Game/UI/WBP_PlayerHUD.UpdateObjectiveTargets` (`self.HUDRef`) _result))))
      (:`then_1`
        (if (== (`self.NbTargetsComplete`) (`KismetArrayLibrary.Array_Length` (`self.CurTargets`)))
          (`self.OnObjectiveComplete`))))))

(fn `RegisterTarget`
  (params (Target :type "/Game/Objectives/BPC_ObjectiveTarget Object Reference") (Type :type "/Game/Objectives/_Enums/EObjectiveType Enum" :default "NewEnumerator0"))
  (`|ExecutionSequence`
    (:`then_0`
      (`/Game/Objectives/BPC_ObjectiveTarget.InitTarget` Target Type))
    (:`then_1`
      (add `/Game/Objectives/BPC_ObjectiveTarget.EvtDispatcher_OnTargetComplete` Target (`|CreateDelegate` :!event `OnTargetComplete`)))))

(fn `StartObjective`
  (params (ObjectiveIndex :type Integer))
  (bind (_type _title _description _targets) (break `/Game/Objectives/_Structs/FObjective` (`|GetArrayItem` (`self.Objectives`) ObjectiveIndex)))
  (`|ExecutionSequence`
    (:`then_0`
      (set `self.NbTargetsComplete` 0))
    (:`then_1`
      (`KismetArrayLibrary.Array_Clear` (`self.CurTargets`)))
    (:`then_2`
      (for _array_element _targets
        (bind _returnvalue (`self.GetComponentByClass` _array_element "/Game/Objectives/BPC_ObjectiveTarget.BPC_ObjectiveTarget_C"))
        (`/Engine/EditorBlueprintResources/StandardMacros.IsValid` _returnvalue
          (:`Is Valid`
            (`KismetArrayLibrary.Array_Add` (`self.CurTargets`) _returnvalue))))
      (`/Game/UI/WBP_PlayerHUD.StartObjective` (`self.HUDRef`) _type _title _description (`KismetArrayLibrary.Array_Length` (`self.CurTargets`))))))

(fn `UserConstructionScript`)