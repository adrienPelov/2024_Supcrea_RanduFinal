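; Base hackable interactible that starts a hacking minigame and unlocks linked interactibles when the player succeeds.
; Interaction start picks settings by difficulty, turns on hacking mode in BP_PlayerController and binds to the HUD widget's success and failure dispatchers.
; Success unlocks InteractiblesToActivate, exits hacking mode and ends the interaction, marking the target hacked.
; Failure only exits hacking mode.
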(event `self.ReceiveTick`
  (params (DeltaSeconds :type "Float (single-precision)"))
  (`parent.ReceiveTick` DeltaSeconds))

(fn `GetInteractionText`
  (returns (Text :type String))
  (return (`KismetStringLibrary.Concat_StrStr` "HACK | " (`self.InteractionText`))))

(fn `OnHackingFailed`
  (bind _asbp_player_controller (cast `/Game/Player/BP_PlayerController` (`Pawn.GetController` (`self.PlayerInTrigger`))))
  (`/Game/Player/BP_PlayerController.ActivateHackingMode` :`self` _asbp_player_controller))

(fn `OnHackingSuccess`
  (for _array_element (`self.InteractiblesToActivate`)
    (`/Engine/EditorBlueprintResources/StandardMacros.IsValid` _array_element
      (:`Is Valid`
        (`self.UnlockInteraction` _array_element true))))
  (bind _asbp_player_controller (cast `/Game/Player/BP_PlayerController` (`Pawn.GetController` (`self.PlayerInTrigger`))))
  (`/Game/Player/BP_PlayerController.ActivateHackingMode` :`self` _asbp_player_controller)
  (`self.OnInteractionEnd`))

(fn `OnInteractionEnd`
  (set `self.bIsHacked` true)
  (`parent.OnInteractionEnd`))

(fn `OnInteractionStart`
  (locals (L_settings :type "/Game/Hacking/_Structs/FHackingSetting Structure"))
  (bind _hudwidget (`/Game/Player/BP_Player.HUDWidget` (`self.PlayerInTrigger`)))
  (`parent.OnInteractionStart`)
  (switch `/Game/Hacking/_Enums/EHackingDifficulty` (`self.Difficulty`)
    (:`NewEnumerator0`
      (set `local.L_settings` (`self.SettingsEasy`)))
    (:`NewEnumerator1`
      (set `local.L_settings` (`self.SettingsMedium`)))
    (:`NewEnumerator2`
      (set `local.L_settings` (`self.SettingsHard`))))
  (bind _asbp_player_controller (cast `/Game/Player/BP_PlayerController` (`GameplayStatics.GetPlayerController` 0)))
  (`/Game/Player/BP_PlayerController.ActivateHackingMode` _asbp_player_controller true (`local.L_settings`))
  (`|ExecutionSequence`
    (:`then_0`
      (add `/Game/UI/WBP_PlayerHUD.EvtDispatcher_HackingSuccess` _hudwidget (`|CreateDelegate` :!event `OnHackingSuccess`)))
    (:`then_1`
      (add `/Game/UI/WBP_PlayerHUD.EvtDispatcher_HackingFailed` _hudwidget (`|CreateDelegate` :!event `OnHackingFailed`)))))

(fn `UserConstructionScript`
  (`parent.UserConstructionScript`))