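; Interactable chest that is marked as hacked when interaction ends, swinging its lid open and awarding score.
; OnInteractionEnd extends the parent's logic, then ChestCompleted rotates the lid root and sends PointsToAdd plus CurrentScore to the HUD.
; Tick retries fetching the HUD widget from the first BP_Player until the reference is valid.
; InitScore and InitTopRotation reset state and lid, but nothing here calls them.
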(event `self.ReceiveTick`
  (params (DeltaSeconds :type "Float (single-precision)"))
  (`parent.ReceiveTick` DeltaSeconds)
  (`self.HUDRef`
    (:`then`)
    (:`else`
      (bind _outactors (`GameplayStatics.GetAllActorsOfClass` "/Game/Player/BP_Player.BP_Player_C"))
      (bind _output (`|GetArrayItem` _outactors))
      (`/Engine/EditorBlueprintResources/StandardMacros.IsValid` _output
        (:`Is Valid`
          (set `self.HUDRef` (`/Game/Player/BP_Player.HUDWidget` _output)))))))

(fn `ChestCompleted`
  (if (`self.ChestHacked`)
    (`SceneComponent.K2_SetRelativeRotation` (`self.Chest_Top_Root`) (struct :`Pitch` 70.0) false false)
    (`/Game/UI/WBP_PlayerHUD.UpdateScore` (`self.HUDRef`) (+ (`self.PointsToAdd`) (`self.CurrentScore`)))))

(fn `InitScore`
  (set `self.CurrentScore` 0)
  (set `self.ChestHacked` false))

(fn `InitTopRotation`
  (`SceneComponent.K2_SetRelativeRotation` :`self` (`self.Chest_Top_Root`)))

(fn `OnInteractionEnd`
  (`parent.OnInteractionEnd`)
  (set `self.ChestHacked` true)
  (`self.ChestCompleted`))

(fn `UserConstructionScript`
  (`parent.UserConstructionScript`))