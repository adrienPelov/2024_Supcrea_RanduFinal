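; BP_Elevator is an elevator whose platform visual moves between a down and an up relative position.
; Evt_Up plays a timeline that lerps the platform between them, Evt_Down reverses it, and BeginPlay scales its rate by TimeToRaise.
; IntPosition reads PositionDown from TargetUp and PositionUp from InteruptorDown, then snaps the platform per IsElevatorUp, but nothing here calls it.
; Interaction start and end only call the parent.
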(event `self.ReceiveBeginPlay`
  (`parent.ReceiveBeginPlay`)
  (`self.Int_Time`))

(event `Evt_Up`
  (bind (_direction _interpolation) (`Timeline|TimelineElevatorRaise` :!label _label)
    (:`Update`
      (`SceneComponent.K2_SetRelativeLocation` (`self.VisuelRootPlateforme`) (`KismetMathLibrary.VLerp` (`self.PositionDown`) (`self.PositionUp`) _interpolation) false false))))

(event `Evt_Down`
  (goto _label :!via `Reverse`))

(fn `Int_Position`
  (bind _visuelrootplateforme (`self.VisuelRootPlateforme`))
  (`|ExecutionSequence`
    (:`then_0`
      (set `self.PositionDown` (`SceneComponent.RelativeLocation` (`self.TargetUp`))))
    (:`then_1`
      (set `self.PositionUp` (`SceneComponent.RelativeLocation` (`self.Interuptor_Down`))))
    (:`then_2`
      (if (`self.bIsElevatorUp`)
        (`SceneComponent.K2_SetRelativeLocation` _visuelrootplateforme (`self.PositionUp`) false false)
        (else
          (`SceneComponent.K2_SetRelativeLocation` _visuelrootplateforme (`self.PositionDown`) false false))))))

(fn `Int_Time`
  (`TimelineComponent.SetPlayRate` (`self.TimelineElevatorRaise`) (/ 1.0 (`self.TimeToRaise`))))

(fn `OnInteractionEnd`
  (`parent.OnInteractionEnd`))

(fn `OnInteractionStart`
  (`parent.OnInteractionStart`))

(fn `UserConstructionScript`
  (`parent.UserConstructionScript`))