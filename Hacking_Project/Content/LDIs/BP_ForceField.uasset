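; BP_ForceField is a force field barrier that can be temporarily disabled by hacking.
; While IsHacked is true, it shows a deactivated material, turns off collision and counts up to MaxTimeDisabled, then clears the flag and restores the active material.
; Tick drives both the timer and an EnableTrigger override, which calls the parent and sets collision from the hacked state.
; The hacked flag is only reset here, never set.
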(event `self.ReceiveBeginPlay`
  (`parent.ReceiveBeginPlay`)
  (`self.Init bIsHacked`)
  (`self.InitTimeDisabled`))

(event `self.ReceiveTick`
  (params (DeltaSeconds :type "Float (single-precision)"))
  (`parent.ReceiveTick` DeltaSeconds)
  (`self.UpdateTimeDisabled` DeltaSeconds)
  (`self.EnableTrigger` true))

(fn `EnableTrigger`
  (params (bEnable :type Boolean))
  (bind _visual_forcefield (`self.Visual_ForceField`))
  (`parent.EnableTrigger` bEnable)
  (if (`self.bIsHacked`)
    (`PrimitiveComponent.SetCollisionEnabled` _visual_forcefield "NoCollision")
    (`self.UpdateTimeDisabled` 0.0)
    (else
      (`PrimitiveComponent.SetCollisionEnabled` _visual_forcefield "QueryAndPhysics"))))

(fn `Init bIsHacked`
  (set `self.bIsHacked` false))

(fn `InitTimeDisabled`
  (set `self.CurrentTimeDisabled` 0.0))

(fn `UpdateTimeDisabled`
  (params (DeltaSeconds :type "Float (double-precision)"))
  (bind _maxtimedisabled (`self.MaxTimeDisabled`))
  (if (`self.bIsHacked`)
    (`PrimitiveComponent.SetMaterial` (`self.Visual_ForceField`) 0 "/Game/Materials/ForceFieldDeactivated.ForceFieldDeactivated")
    (bind _output_get (set `self.CurrentTimeDisabled` (`KismetMathLibrary.FClamp` (+ DeltaSeconds (`self.CurrentTimeDisabled`)) 0.0 _maxtimedisabled)))
    (if (== _output_get _maxtimedisabled)
      (set `self.bIsHacked` false)
      (`PrimitiveComponent.SetMaterial` (`self.Visual_ForceField`) 0 "/Game/Materials/ForceField.ForceField"))
    (else
      (set `self.CurrentTimeDisabled` 0.0))))

(fn `UserConstructionScript`
  (`parent.UserConstructionScript`))