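; BP_SwitchElevator is an interactable switch that remotely triggers the elevators referenced in its InterractElevator array.
; Its TryInteract override runs the parent behavior, then calls UnlockInteraction and OnInteractionStart on each valid array entry, so one use both unlocks and starts them.
; The event graph and construction script add no logic of their own.
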(fn `TryInteract`
  (`parent.TryInteract`)
  (for _array_element (`self.InterractElevator`)
    (`/Engine/EditorBlueprintResources/StandardMacros.IsValid` _array_element
      (:`Is Valid`
        (`self.UnlockInteraction` _array_element true)
        (`self.OnInteractionStart` _array_element)))))

(fn `UserConstructionScript`
  (`parent.UserConstructionScript`))